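; Arcanoid bonus pickup that moves along the Y axis each tick and destroys itself on overlapping a KillZVolume.
; The construction script picks one of seven bonus types at random, using DebuffThreshold to weight the four debuffs against the three buffs, and shows the type's name on its TextRender.
; Movement is swept and scaled by Direction and Speed; applying the bonus effect is not handled here.
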(event EventBeginPlay)

(event Collision|EventActorBeginOverlap
  (params (OtherActor :type Actor%20Object%20Reference))
  (Utilities|Casting|CastToKillZVolume OtherActor)
  (Actor|DestroyActor))

(event EventTick
  (params (DeltaSeconds :type Float%20%28single-precision%29))
  (Transformation|AddActorWorldOffset (Math|Vector|MakeVector 0.0 (.y (* (Variables|Default|GetDirection) (* DeltaSeconds (Variables|Default|GetSpeed)))) 0.0) true))

(fn ConstructionScript
  (bind _buffoption (CallFunction|GetBuffOption (Math|Random|RandomIntegerinRange 0 100)))
  (Variables|Default|SetBonusType (Utilities|Select :Index _buffoption :Option%200 "NewEnumerator0" :Option%201 "NewEnumerator1" :Option%202 "NewEnumerator2" :Option%203 "NewEnumerator3" :Option%204 "NewEnumerator4" :Option%205 "NewEnumerator5" :Option%206 "NewEnumerator6"))
  (Rendering|Components|TextRender|SetText (Variables|Default|GetTextRender) (Utilities|Text|ToText(String) (Utilities|String|EnumtoString (Variables|Default|GetBonusType)))))

(fn GetBuffOption
  (params (RandomNumber :type Integer))
  (if (<= RandomNumber (Variables|Default|GetDebuffThreshold))
    (Variables|Default|SetBuffOption (Math|Random|RandomIntegerinRange 3 6))
    (else
      (Variables|Default|SetBuffOption (Math|Random|RandomIntegerinRange 0 2))))
  (return (Variables|Default|GetBuffOption)))