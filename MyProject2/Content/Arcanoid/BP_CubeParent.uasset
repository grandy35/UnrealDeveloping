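; BP_CubeParent is a base brick for an Arkanoid-style game that takes damage when hit by the ball.
; A Hit from BP_Ball calls BallisHit, which decrements Lives and either destroys the brick at zero or below or switches its material to steel.
; The Construction Script gives bricks with two lives a moss material, so their starting durability is visible.
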(event Custom|BallisHit
  (bind _result (Math|Integer|DecrementInt (Variables|Default|GetLives))
    (:%20%20
      (if (<= _result 0)
        (Actor|DestroyActor)
        (else
          (Rendering|Material|SetMaterial (Variables|Default|GetCube) 0 "/Game/StarterContent/Materials/M_Metal_Steel.M_Metal_Steel"))))))

(event EventBeginPlay)

(event Collision|EventActorBeginOverlap
  (params (OtherActor :type Actor%20Object%20Reference)))

(event EventTick
  (params (DeltaSeconds :type Float%20%28single-precision%29)))

(event Collision|EventHit
  (params (MyComp :type Primitive%20Component%20Object%20Reference) (Other :type Actor%20Object%20Reference) (OtherComp :type Primitive%20Component%20Object%20Reference) (bSelfMoved :type Boolean) (HitLocation :type Vector :default "0, 0, 0") (HitNormal :type Vector :default "0, 0, 0") (NormalImpulse :type Vector :default "0, 0, 0") (Hit :type Hit%20Result%20Structure%20%28by%20ref%29))
  (Utilities|Casting|CastToBP_Ball Other)
  (CallFunction|BallisHit))

(fn ConstructionScript
  (bind _output_get (Variables|Default|SetLives (Variables|Default|GetLives)))
  (switch int _output_get
    (:2
      (Rendering|Material|SetMaterial (Variables|Default|GetCube) 0 "/Game/StarterContent/Materials/M_Ground_Moss.M_Ground_Moss"))))