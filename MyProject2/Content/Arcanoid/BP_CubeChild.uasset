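; BP_CubeChild is a cube variant for the Arcanoid game that can drop a bonus when destroyed.
; On BeginPlay it binds its OnDestroyed event to SpawnBonus, which uses a weighted random roll to occasionally spawn a scaled-down, rotated BP_bonus at the cube's location.
; Ball hit handling and construction only call the parent implementation.
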(event Custom|SpawnBonus
  (params (DestroyedActor :type Actor%20Object%20Reference))
  (if (Math|Random|RandomBoolwithWeight 0.3)
    (Game|SpawnActorfromClass "/Game/Arcanoid/Bonuses/BP_bonus.BP_bonus_C" (Math|Transform|MakeTransform (Transformation|GetActorLocation) "0, 0,90.000000" "0.500000,0.500000,0.500000") "AlwaysSpawn" 0 0)))

(event EventBeginPlay
  (EventDispatchers|BindEventtoOnDestroyed (delegate Custom|SpawnBonus)))

(event EventBallisHit
  (|CallParentFunction))

(fn ConstructionScript
  (|CallParentFunction))