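; BP_Generator is an Arcanoid actor that spawns a grid of BP_CubeChild cubes, sized by X, Y and Padding.
; The construction script builds a static mesh preview of the grid, which BeginPlay destroys before spawning the cubes from the actor's location into CubesArray.
; GetCubesforWin returns that array's length.
; Tick moves only the generator vertically with sweep, by Direction and Speed, as spawned cubes are not attached.
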(event EventBeginPlay
  (bind _returnvalue (Transformation|GetActorLocation))
  (for _array_element (Variables|Default|GetPreviewArray)
    (Components|DestroyComponent _array_element))
  (for _index (range 0 (Variables|Default|GetX))
    (for _index_2 (range 0 (Variables|Default|GetY))
      (bind _returnvalue_2 (Game|SpawnActorfromClass "/Game/Arcanoid/BP_CubeChild.BP_CubeChild_C" (Math|Transform|MakeTransform (Math|Vector|MakeVector (+ (.x _returnvalue) (Math|Conversions|ToFloat(Integer) (* _index (Variables|Default|GetPadding)))) (+ (.y _returnvalue) (Math|Conversions|ToFloat(Integer) (* _index_2 (Variables|Default|GetPadding)))) (.z _returnvalue))) "Undefined" 0 0))
      (Utilities|Array|Add (Variables|Default|GetCubesArray) _returnvalue_2))))

(event EventTick
  (params (DeltaSeconds :type Float%20%28single-precision%29))
  (Transformation|AddActorWorldOffset (Math|Vector|MakeVector 0.0 0.0 (.z (* (Variables|Default|GetDirection) (* DeltaSeconds (Variables|Default|GetSpeed))))) true))

(fn ConstructionScript
  (for _index (range 0 (Variables|Default|GetX))
    (for _index_2 (range 0 (Variables|Default|GetY))
      (bind _returnvalue (AddComponent|AddStaticMeshComponent false (Math|Transform|MakeTransform (Math|Vector|MakeVector (Math|Conversions|ToFloat(Integer) (* _index (Variables|Default|GetPadding))) (Math|Conversions|ToFloat(Integer) (* _index_2 (Variables|Default|GetPadding))) 0.0))))
      (Utilities|Array|Add (Variables|Default|GetPreviewArray) _returnvalue))))

(fn GetCubesforWin
  (return (Utilities|Array|Length (Variables|Default|GetCubesArray))))